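; Player hero Blueprint that handles interaction with overlapping actors and end-of-game win or lose presentation.
; Overlaps show or hide interact pop-ups through interface messages, and Interact input messages every overlapping actor, tracking results for pop-up cleanup.
; Celebrate and Lose spawn a camera at VictoryCamPosition, blend to it, loop their animation and lock BP_GMCPlayerController movement and actions.
; The construction script removes weapon components when no mesh is set.
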(event Custom|Celebrate
  (bind _returnvalue (Game|SpawnActorfromClass "/Script/Engine.CameraActor" (Transformation|GetWorldTransform (Variables|Default|GetVictoryCamPosition)) "Undefined" (Game|GetPlayerController 0) 0))
  (Game|Player|SetViewTargetwithBlend (Game|GetPlayerController 0) _returnvalue 0.0 "VTBlend_Linear" 0.0 false)
  (Components|Animation|PlayAnimation (Variables|Character|GetMesh) (Variables|Default|GetCelebrateMontage) true)
  (bind _asbp_gmcplayer_controller (Utilities|Casting|CastToBP_GMCPlayerController (Game|GetPlayerController 0)))
  (Class|GMCPlayerController|LockPlayerMovement _asbp_gmcplayer_controller true)
  (Class|GMCPlayerController|LockPlayerActions _asbp_gmcplayer_controller true))

(event Custom|Lose
  (bind _returnvalue (Game|SpawnActorfromClass "/Script/Engine.CameraActor" (Transformation|GetWorldTransform (Variables|Default|GetVictoryCamPosition)) "Undefined" (Game|GetPlayerController 0) 0))
  (Game|Player|SetViewTargetwithBlend (Game|GetPlayerController 0) _returnvalue 0.0 "VTBlend_Linear" 0.0 false)
  (Components|Animation|PlayAnimation (Variables|Character|GetMesh) (Variables|Default|GetLoseMontage) true)
  (bind _asbp_gmcplayer_controller (Utilities|Casting|CastToBP_GMCPlayerController (Game|GetPlayerController 0)))
  (Class|GMCPlayerController|LockPlayerMovement _asbp_gmcplayer_controller true)
  (Class|GMCPlayerController|LockPlayerActions _asbp_gmcplayer_controller true))

(event Collision|EventActorEndOverlap
  (params (OtherActor :type Actor%20Object%20Reference))
  (Class|BPIInteractInterface|HideInteractPopUp(Message) OtherActor self)
  (for _array_element (Variables|Default|GetInteractedActors)
    (Class|BPIInteractInterface|HideInteractPopUp(Message) _array_element))
  (Utilities|Array|Clear (Variables|Default|GetInteractedActors)))

(event Collision|EventActorBeginOverlap
  (params (OtherActor :type Actor%20Object%20Reference))
  (Class|BPIInteractInterface|DisplayInteractPopUp(Message) OtherActor self))

(event Input|ActionEvents|InputActionInteract
  (params (Key :type Key%20Structure :default "None"))
  ;[1 1 1] Looks for overlapping actors and tries to call their Interact Interface
  (:Pressed
    (for _array_element (Collision|GetOverlappingActors 0 :!class /Script/Engine.Actor)
      (bind _interactedactor (Class|BPIInteractInterface|Interact(Message) _array_element self))
      (Utilities|Array|AddUnique (Variables|Default|GetInteractedActors) _interactedactor))))

(fn ConstructionScript
  (Utilities|IsValid (Variables|/Script/Engine.StaticMeshComponent|GetStaticMesh (Variables|Default|GetWeapon))
    (:Is%20Not%20Valid
      (Components|DestroyComponent (Variables|Default|GetWeapon)))))

(fn DisplayInteractPopUp
  (params (Caller :type Actor%20Object%20Reference))
  (return false))

(fn HideInteractPopUp
  (params (Caller :type Actor%20Object%20Reference))
  (return false))

(fn Interact
  (params (CallingActor :type Actor%20Object%20Reference))
  (return 0))