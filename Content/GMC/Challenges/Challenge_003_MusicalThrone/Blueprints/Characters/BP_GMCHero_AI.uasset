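; AI hero character for the Musical Throne challenge, shown as a red, blue or green knight.
; The construction script sets the mesh material from its team color.
; On BeginPlay it stores its starting transform for ResetToStarting to teleport back to, and binds OnFadeOut to the challenge game mode, deferring to the parent's handling.
; Losing plays a one-shot lose animation on the mesh.
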(event Custom|OnLose
  (Components|Animation|PlayAnimation (Variables|Character|GetMesh) "/Game/GMC/Challenges/Challenge_003_MusicalThrone/Animations/Anim_Lose.Anim_Lose" false))

(event EventBeginPlay
  (Variables|Default|SetStartingPosition (Transformation|GetActorTransform))
  (bind _asbp_gmcgame_mode_003 (Utilities|Casting|CastToBP_GMCGameMode_003 (Game|GetGameMode)))
  (EventDispatchers|BindEventtoOnFadeOut _asbp_gmcgame_mode_003 (delegate EventOnFadeOut)))

(event EventOnFadeOut
  (|CallParentFunction))

(fn ConstructionScript
  (CallFunction|SetTeamColor))

(fn ResettoStarting
  (bind _startingposition (Variables|Default|GetStartingPosition))
  (Transformation|SetActorTransform (Math|Transform|MakeTransform (.location _startingposition) (.rotation _startingposition) "1,1,1") false true))

(fn SetTeamColor
  (bind _mesh (Variables|Character|GetMesh))
  (switch Utilities|FlowControl|Switch|SwitchonETeamColor (Variables|Default|GetTeamColor)
    (:NewEnumerator0
      (Rendering|Material|SetMaterial _mesh 0 (Variables|Default|GetRedKnight)))
    (:NewEnumerator1
      (Rendering|Material|SetMaterial _mesh 0 (Variables|Default|GetBlueKnight)))
    (:NewEnumerator2
      (Rendering|Material|SetMaterial _mesh 0 (Variables|Default|GetGreenKnight)))))