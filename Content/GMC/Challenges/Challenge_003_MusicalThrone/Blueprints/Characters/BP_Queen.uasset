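; BP_Queen is the interactable Queen character in the Musical Throne challenge, which the player can talk to.
; Display and hide functions drive the GMCInteractable pop-up, and displaying it enables interaction.
; Interacting opens a WBP_003_DialogueBox, blends the view to the Queen, locks player movement and actions, and switches to mouse-driven UI input.
; It also binds to the challenge game mode's fade-out event to destroy its Box component.
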(event OnInteract(GMCInteractable))

(event Custom|OnGameStarted
  (bind _box (Variables|Default|GetBox))
  (Utilities|IsValid _box
    (:Is%20Valid
      (Components|DestroyComponent _box))))

(event EventBeginPlay
  (bind _asbp_gmcgame_mode_003 (Utilities|Casting|CastToBP_GMCGameMode_003 (Game|GetGameMode)))
  (EventDispatchers|BindEventtoOnFadeOut _asbp_gmcgame_mode_003 (delegate Custom|OnGameStarted)))

(fn ConstructionScript)

(fn DisplayInteractPopUp
  (params (Caller :type Actor%20Object%20Reference))
  (Class|GMCInteractableComponent|CallDisplayPopUp (Variables|Default|GetGMCInteractable))
  (bind _output_get (Variables|Default|SetCanInteract true))
  (return _output_get))

(fn HideInteractPopUp
  (params (Caller :type Actor%20Object%20Reference))
  (Class|GMCInteractableComponent|CallHidePopUp (Variables|Default|GetGMCInteractable))
  (return false))

(fn Interact
  (params (CallingActor :type Actor%20Object%20Reference))
  (if (Variables|Default|GetCanInteract)
    (Class|GMCInteractableComponent|CallInteract (Variables|Default|GetGMCInteractable))
    (bind _asbp_gmcplayer_controller (Utilities|Casting|CastToBP_GMCPlayerController (Game|GetPlayerController 0)))
    (bind _output_get (Variables|Default|SetGMCController _asbp_gmcplayer_controller))
    (bind _returnvalue (UserInterface|CreateWidget "/Game/GMC/Challenges/Challenge_003_MusicalThrone/UI/WBP_003_DialogueBox.WBP_003_DialogueBox_C" _output_get 2e+01 self))
    (bind _output_get_2 (Variables|Default|SetDialogueWidget _returnvalue))
    (UserInterface|Viewport|AddtoViewport _output_get_2 0)
    (CallFunction|HideInteractPopUp)
    (Game|Player|SetViewTargetwithBlend (Variables|Default|GetGMCController) self 0.0 "VTBlend_Linear" 0.0 false)
    (Class|GMCPlayerController|LockPlayerMovement (Variables|Default|GetGMCController) true)
    (Class|GMCPlayerController|LockPlayerActions (Variables|Default|GetGMCController) true)
    (Variables|/Script/Engine.PlayerController|SetbShowMouseCursor (Variables|Default|GetGMCController) true)
    (Input|SetInputModeGameandUI (Variables|Default|GetGMCController) (Variables|Default|GetDialogueWidget) "DoNotLock" true)
    (Variables|Default|SetCanInteract false)
    (return self)))