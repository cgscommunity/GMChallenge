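; Player hero character Blueprint for GMC Challenge 003, Musical Throne.
; On BeginPlay it binds to the fade-out event of BP_GMCGameMode_003, which clears the Sitting state and restores query and physics collision on the capsule and mesh.
; The DialogueAutoComplete input action triggers CallDialogueAutoComplete, and construction only runs the parent script.
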(event Custom|OnFadeOut
  (Variables|Default|SetbSitting false)
  (Collision|SetCollisionEnabled (Variables|Default|GetCapsuleComponent) "QueryAndPhysics"))

(event EventBeginPlay
  (bind _asbp_gmcgame_mode_003 (Utilities|Casting|CastToBP_GMCGameMode_003 (Game|GetGameMode)))
  (EventDispatchers|BindEventtoOnFadeOut _asbp_gmcgame_mode_003 (delegate Custom|OnFadeOut)))

(event Input|ActionEvents|InputActionDialogueAutoComplete
  (params (Key :type Key%20Structure :default "None"))
  (:Pressed
    (Default|CallDialogueAutoComplete)))

(fn ConstructionScript
  (|CallParentFunction))