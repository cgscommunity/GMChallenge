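; Wall and rotating base for the Musical Throne challenge, driven by the game mode's music start, stop and fade-out events.
; Music start raises the wall and eases the base into a timer-looped spin; music stop eases it out and lowers the wall.
; Fade-out clears tracked chairs, rebuilds spawn points from child components and calls SpawnChairs, an unfinished stub spawning one chair at the first point.
; RemoveRandomChair exists but is never called here.
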(event Custom|ToggleSpin
  (params (ShouldSpin :type Boolean))
  (if ShouldSpin
    (Variables|Default|SetbIsSpinning true)
    (bind _rotationmultiplier (Timeline|SpinEase PlayFromStart)
      (:Update
        (CallFunction|RotateBase (* _rotationmultiplier (Variables|Default|GetRotationAmount))))
      (:Finished
        (CallFunction|Spin)))
    (else
      (Variables|Default|SetbIsSpinning false)
      (Timeline|SpinEase ReverseFromEnd))))

(event Custom|AnimateWall
  (params (AnimateDown :type Boolean))
  (Audio|PlaySoundatLocation "/Game/GMC/Challenges/Challenge_003_MusicalThrone/Audio/heavy-stone-push.heavy-stone-push" (Transformation|GetWorldLocation (Variables|Default|GetWall)) "0, 0, 0" 0.5 1.0 0.0 0 0 0)
  (if AnimateDown
    (bind _zposition (Timeline|WallAnimation PlayFromStart)
      (:Update
        (Transformation|SetRelativeLocation (Variables|Default|GetWall) (Math|Vector|MakeVector 0.0 0.0 _zposition) false false)))
    (else
      (Timeline|WallAnimation ReverseFromEnd))))

(event Custom|OnStartMusic
  (CallFunction|AnimateWall false)
  (Utilities|FlowControl|Delay 0.6)
  (CallFunction|ToggleSpin true))

(event Custom|OnStopMusic
  (Variables|Default|SetOccupiedChairs 0)
  (CallFunction|ToggleSpin false)
  (CallFunction|AnimateWall true))

(event Custom|OnFadeOut
  (CallFunction|DestroyChairs)
  (CallFunction|SetupSpawnPoints)
  (CallFunction|SpawnChairs))

(event EventBeginPlay
  (bind _asbp_gmcgame_mode_003 (Utilities|Casting|CastToBP_GMCGameMode_003 (Game|GetGameMode)))
  (Variables|Default|SetGameMode_003 _asbp_gmcgame_mode_003)
  (CallFunction|SetupBindings))

(fn ConstructionScript)

(fn RotateBase
  (params (RotationAmount :type Float%20%28single-precision%29))
  (bind _base (Variables|Default|GetBase))
  (bind _relativerotation (Variables|/Script/Engine.SceneComponent|GetRelativeRotation _base))
  (Transformation|SetRelativeRotation (Variables|Default|GetBase) (Math|Rotator|MakeRotator (.roll _relativerotation) (.pitch _relativerotation) (+ (.yaw _relativerotation) RotationAmount)) false false))

(fn Spin
  (if (Variables|Default|GetbIsSpinning)
    (CallFunction|RotateBase (Variables|Default|GetRotationAmount))
    (Utilities|Time|SetTimerbyFunctionName 0 "Spin" (Variables|Default|GetSpinSpeed))))

(fn SetupBindings
  (bind _gamemode_003 (Variables|Default|GetGameMode_003))
  (EventDispatchers|BindEventtoOnStartMusic _gamemode_003 (EventDispatchers|CreateEvent :!event Custom|OnStartMusic))
  (EventDispatchers|BindEventtoOnStopMusic _gamemode_003 (EventDispatchers|CreateEvent :!event Custom|OnStopMusic))
  (EventDispatchers|BindEventtoOnFadeOut _gamemode_003 (EventDispatchers|CreateEvent :!event Custom|OnFadeOut)))

(fn SpawnChairs
  ;[1 1 1] Hint: Use this function to spawn charis at the different points. Be sure to remove a chair for each round and spawn the Throne in the end.
  (Game|SpawnActorfromClass "/Game/GMC/Challenges/Challenge_003_MusicalThrone/Blueprints/BP_Chair.BP_Chair_C" (Utilities|Array|Get(acopy) (Variables|Default|GetChairSpawnPoints)) "Undefined" 0 0))

(fn DestroyChairs
  (bind _activechairs (Variables|Default|GetActiveChairs))
  (if (> (Utilities|Array|Length _activechairs) 0)
    (for _array_element _activechairs
      (Actor|DestroyActor _array_element))
    (Utilities|Array|Clear (Variables|Default|GetActiveChairs))))

(fn SetupSpawnPoints
  (Utilities|Array|Clear (Variables|Default|GetChairSpawnPoints))
  (for _array_element (Components|GetChildrenComponents (Variables|Default|GetChairs) false)
    (Utilities|Array|AddUnique (Variables|Default|GetChairSpawnPoints) (Transformation|GetWorldTransform _array_element))))

(fn RemoveRandomChair
  (bind _chairspawnpoints (Variables|Default|GetChairSpawnPoints))
  (Utilities|Array|RemoveItem (Variables|Default|GetChairSpawnPoints) (Utilities|Array|Get(acopy) _chairspawnpoints (Math|Random|RandomIntegerinRange 0 (- (Utilities|Array|Length _chairspawnpoints) 1)))))