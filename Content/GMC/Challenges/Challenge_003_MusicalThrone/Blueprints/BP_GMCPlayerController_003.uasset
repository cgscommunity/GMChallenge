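; Player controller for the Musical Throne challenge (003) that holds players still during the pre-game countdown.
; On BeginPlay it runs the parent logic, then binds to the challenge game mode's fade-out and game-started events.
; Fade-out marks the countdown start and locks player movement, and game start unlocks it.
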(event Custom|OnCountdownStart
  (Class|GMCPlayerController|LockPlayerMovement true))

(event Custom|OnGameStart
  (Class|GMCPlayerController|LockPlayerMovement false))

(event EventBeginPlay
  (|CallParentFunction)
  (bind _asbp_gmcgame_mode_003 (Utilities|Casting|CastToBP_GMCGameMode_003 (Game|GetGameMode)))
  (EventDispatchers|BindEventtoOnFadeOut _asbp_gmcgame_mode_003 (delegate Custom|OnCountdownStart))
  (EventDispatchers|BindEventtoOnGameStarted _asbp_gmcgame_mode_003 (delegate Custom|OnGameStart)))

(fn ConstructionScript
  (|CallParentFunction))