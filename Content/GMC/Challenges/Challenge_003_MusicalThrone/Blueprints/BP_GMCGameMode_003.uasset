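; Game mode for a musical chairs challenge (Musical Throne) that runs the countdown, music cycle and game-over celebration.
; Setup spawns music and HUD and gathers the player and AI; screen fades frame countdown and game over.
; Music pauses after a random timer, with event dispatchers broadcasting each phase.
; AllChairsOccupied is an empty stub for round-loser logic, and nothing here calls StartCountdown or GameOver.
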(event Custom|GameOver
  (params (Winner :type Actor%20Object%20Reference))
  (Variables|Default|SetbGameOver true)
  (CallFunction|FadeOut)
  (Utilities|FlowControl|Delay (Variables|Default|GetFadeTime))
  (bind _ascharacter (Utilities|Casting|CastToCharacter Winner))
  (Default|CallOnGameOver _ascharacter)
  (Utilities|FlowControl|Delay 0.2)
  (CallFunction|Fadein)
  (bind _returnvalue (Audio|CreateSound2D "/Game/GMC/Challenges/Challenge_003_MusicalThrone/Audio/WinningCelebration.WinningCelebration" 1.0 1.0 0.0 0))
  (Audio|Components|Audio|FadeIn _returnvalue 0.5 1.0 0.0 "Linear" :!class /Script/Engine.AudioComponent))

(event Custom|StartCountdown
  (bind _countdowntimestart (Variables|Default|GetCountdownTimeStart))
  ;[1 1 1] Hint: Use this event at the start of every round
  (CallFunction|FadeOut)
  (Utilities|FlowControl|Delay (Variables|Default|GetFadeTime))
  (Default|CallOnFadeOut)
  (Utilities|FlowControl|Delay 0.2)
  (CallFunction|Fadein)
  (Audio|PlaySound2D "/Game/GMC/Challenges/Challenge_003_MusicalThrone/Audio/trumpet-brass-fanfare.trumpet-brass-fanfare" 1.0 1.0 0.0 0 0)
  (Utilities|FlowControl|Delay (Variables|Default|GetFadeTime))
  (Default|CallOnCountdownStarted _countdowntimestart)
  (Variables|Default|SetCountdownTimeRemaining _countdowntimestart)
  (Utilities|FlowControl|Delay 1.0)
  (CallFunction|TickCountdown))

(event Custom|StartGame
  (Variables|Default|SetbGameOver false)
  (Default|CallOnGameStarted)
  (CallFunction|StartMusic))

(event Custom|StartMusic
  (Variables|Default|SetbMusicPaused false)
  (if (not (Variables|Default|GetbGameOver))
    (Default|CallOnStartMusic)
    (Utilities|FlowControl|Delay 0.6)
    (CallFunction|PlayMusic)
    (Utilities|Time|SetTimerbyEvent (delegate Custom|StopMusic) (Math|Random|RandomFloatinRange 5.0 1e+01))))

(event Custom|StopMusic
  (Variables|Default|SetbMusicPaused true)
  (Default|CallOnStopMusic)
  (CallFunction|PauseMusic))

(event Custom|AllChairsOccupied
  ;[1 1 1] Hint: Have logic for when all chairs are occupied. Determine who the loser of the round is and go from there.
)

(event EventBeginPlay
  (CallFunction|SetupGame))

(fn ConstructionScript)

(fn SetupGame
  (bind _returnvalue (Game|GetPlayerController 0))
  (bind _returnvalue_2 (Audio|SpawnSound2D "/Game/GMC/Challenges/Challenge_003_MusicalThrone/Audio/MusicalChairs.MusicalChairs" 1.0 1.0 0.0 0))
  (Variables|Default|SetMusic _returnvalue_2)
  (bind _returnvalue_3 (UserInterface|CreateWidget "/Game/GMC/Challenges/Challenge_003_MusicalThrone/UI/WBP_HUD_003.WBP_HUD_003_C" _returnvalue))
  (UserInterface|Viewport|AddtoViewport _returnvalue_3 0)
  (Input|SetInputModeGameOnly _returnvalue)
  (Variables|/Script/Engine.PlayerController|SetbShowMouseCursor _returnvalue false)
  (CallFunction|GetPlayers))

(fn PauseMusic
  (Class|AudioComponent|SetPaused (Variables|Default|GetMusic) true)
  (Variables|Default|SetbMusicPaused true))

(fn PlayMusic
  (Utilities|IsValid (Variables|Default|GetMusic)
    (:Is%20Valid
      (Class|AudioComponent|SetPaused (Variables|Default|GetMusic) false)
      (Variables|Default|SetbMusicPaused false))
    (:Is%20Not%20Valid
      (bind _returnvalue (Audio|SpawnSound2D "/Game/GMC/Challenges/Challenge_003_MusicalThrone/Audio/MusicalChairs.MusicalChairs" 1.0 1.0 0.0 0))
      (bind _output_get (Variables|Default|SetMusic _returnvalue))
      (Audio|Components|Audio|Play _output_get 0.0))))

(fn FadeOut
  (bind _returnvalue (UserInterface|CreateWidget "/Game/GMC/GlobalAssets/UI/WBP_ScreenFade.WBP_ScreenFade_C" (Game|GetPlayerController 0)))
  (bind _output_get (Variables|Default|SetFadeScreen _returnvalue))
  (UserInterface|Viewport|AddtoViewport _output_get 0)
  (Variables|Default|SetFadeTime (Class|WidgetAnimation|GetEndTime (Variables|/Game/GMC/GlobalAssets/UI/WBP_ScreenFade.WBP_ScreenFade_C|GetFadeInOut _output_get)))
  (UserInterface|Animation|PlayAnimation _output_get (Variables|/Game/GMC/GlobalAssets/UI/WBP_ScreenFade.WBP_ScreenFade_C|GetFadeInOut _output_get) 0.0 1 "Forward" 1.0 false)
  (if (not (Variables|Default|GetbMusicPaused))
    (Audio|Components|Audio|FadeOut (Variables|Default|GetMusic) (Variables|Default|GetFadeTime) 0.0 "Linear" :!class /Script/Engine.AudioComponent)))

(fn Fadein
  (bind _fadescreen (Variables|Default|GetFadeScreen))
  (Utilities|IsValid _fadescreen
    (:Is%20Valid
      (UserInterface|Animation|PlayAnimation _fadescreen (Variables|/Game/GMC/GlobalAssets/UI/WBP_ScreenFade.WBP_ScreenFade_C|GetFadeInIn _fadescreen) 0.0 1 "Forward" 1.0 false))))

(fn TickCountdown
  (bind _result (Math|Float|DecrementFloat (Variables|Default|GetCountdownTimeRemaining))
    (:%20%20
      (if (> _result 0.0)
        (Utilities|Time|SetTimerbyFunctionName 0 "Tick Countdown" 1.0)
        (Default|CallOnTimerUpdated (Variables|Default|GetCountdownTimeRemaining))
        (Audio|PlaySound2D "/Game/GMC/Challenges/Challenge_003_MusicalThrone/Audio/low_snare.low_snare" 1.0 1.0 0.0 0 0)
        (else
          (CallFunction|StartGame)
          (Default|CallOnGameStarted))))))

(fn GetPlayers
  (bind _asbp_gmchero_003 (Utilities|Casting|CastToBP_GMCHero_003 (Game|Player|GetPlayerPawn 0)))
  (Variables|Default|SetPlayerCharacter _asbp_gmchero_003)
  (bind _outactors (Actor|GetAllActorsOfClass "/Game/GMC/Challenges/Challenge_003_MusicalThrone/Blueprints/Characters/BP_AI_003.BP_AI_003_C"))
  (for _array_element _outactors
    (Utilities|Array|AddUnique (Variables|Default|GetAI_Players) _array_element)))