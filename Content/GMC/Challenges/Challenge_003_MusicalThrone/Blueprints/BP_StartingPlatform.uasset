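; BP_StartingPlatform is a starting platform for the Musical Throne challenge that positions a character at the start.
; The construction script applies a configurable mesh to two flag components.
; On BeginPlay, PlaceCharactersInPosition moves its assigned Character, if valid, to the StartingPosition component's world location and rotation and clears its Sitting flag.
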(event EventBeginPlay
  (CallFunction|PlaceCharactersinPosition))

(fn ConstructionScript
  (bind _flagmesh (Variables|Default|GetFlagMesh))
  (Components|StaticMesh|SetStaticMesh (Variables|Default|GetFlag1) _flagmesh)
  (Components|StaticMesh|SetStaticMesh (Variables|Default|GetFlag2) _flagmesh))

(fn PlaceCharactersinPosition
  (if (Utilities|IsValid (Variables|Default|GetCharacter))
    (Transformation|SetActorLocation (Variables|Default|GetCharacter) (Transformation|GetWorldLocation (Variables|Default|GetStartingPosition)) false false)
    (Transformation|SetActorRotation (Variables|Default|GetCharacter) (Transformation|GetWorldRotation (Variables|Default|GetStartingPosition)))
    (Variables|/Game/GMC/Challenges/Challenge_003_MusicalThrone/Blueprints/Characters/BP_GMCHero_003.BP_GMCHero_003_C|SetbSitting (Variables|Default|GetCharacter) false)))