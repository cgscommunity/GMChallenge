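; Game mode for the Whack-a-Zombie challenge, running a pre-game countdown, a timed round and the ending.
; BeginPlay locks player movement, then chains delays to StartGame and EndGame, while looping one-second timers decrement the countdown values and play start ticks.
; StartGame unlocks movement and EndGame relocks it with a hero celebration, each firing a game event.
; Restart clears the started flag and restarts the game.
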(event Custom|BeginPlayCountdown
  (bind _newtime (CallFunction|CountdownTimer (Variables|Default|GetCurrentStartTime)))
  (bind _output_get (Variables|Default|SetCurrentStartTime _newtime))
  (if (> _output_get 0)
    (Audio|PlaySound2D "/Game/GMC/Challenges/Challenge_001_WhackAZombie/Audio/SFX/tick.tick" 1.0 1.0 0.0 0 0)))

(event Custom|StartGame
  (Variables|Default|SetGameStarted true)
  (Class|GMCPlayerController|LockPlayerMovement (Variables|Default|GetPlayerController) false)
  (Default|CallGameStartEvent))

(event Custom|GameCountdown
  (bind _newtime (CallFunction|CountdownTimer (Variables|Default|GetTimeRemaining)))
  (Variables|Default|SetTimeRemaining _newtime))

(event Custom|EndGame
  (Default|Celebrate (Variables|Default|GetPlayerCharacter))
  (Class|GMCPlayerController|LockPlayerMovement (Variables|Default|GetPlayerController) true)
  (Default|CallGameEndEvent))

(event Custom|Restart
  (Variables|Default|SetGameStarted false)
  (Class|GameMode|RestartGame))

(event EventBeginPlay
  (bind _asbp_gmchero_001 (Utilities|Casting|CastToBP_GMCHero_001 (Game|Player|GetPlayerPawn 0)))
  (Variables|Default|SetPlayerCharacter _asbp_gmchero_001)
  (bind _asbp_gmcplayer_controller (Utilities|Casting|CastToBP_GMCPlayerController (Game|GetPlayerController 0)))
  (bind _output_get (Variables|Default|SetPlayerController _asbp_gmcplayer_controller))
  (Class|GMCPlayerController|LockPlayerMovement _output_get true)
  (Variables|Default|SetCurrentStartTime (Variables|Default|GetStartTime))
  (Utilities|Time|SetTimerbyEvent (delegate Custom|BeginPlayCountdown) 1.0 true)
  (Utilities|FlowControl|Delay (Math|Conversions|ToFloat(Integer) (Variables|Default|GetCurrentStartTime)))
  (CallFunction|StartGame)
  (Variables|Default|SetTimeRemaining (Variables|Default|GetTotalGameTime))
  (Utilities|Time|SetTimerbyEvent (delegate Custom|GameCountdown) 1.0 true)
  (Utilities|FlowControl|Delay (Math|Conversions|ToFloat(Integer) (Variables|Default|GetTotalGameTime)))
  (CallFunction|EndGame))

(fn ConstructionScript)

(fn CountdownTimer
  (params (StartingTime :type Integer))
  (if (> StartingTime 0)
    (return (- StartingTime 1))))