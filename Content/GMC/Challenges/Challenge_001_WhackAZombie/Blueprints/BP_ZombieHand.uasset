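; BP_ZombieHand is the zombie hand actor for the Whack-A-Zombie challenge, left partly unfinished with hint comments.
; On BeginPlay it plays a randomly pitched sound, caches the hand's anim instance and active montage, and creates a dynamic material instance for a hit flash.
; FlashGreen and OnHit are empty stubs, and the node setting the material's EmissiveValue is unconnected, so the flash does not yet run.
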(event Custom|OnHit
  ;[1 1 1] Hint: These were custome events I created.
)

(event Custom|FlashGreen
  ;[1 1 1] Hint: These were custome events I created.
)

(event EventBeginPlay
  (Audio|PlaySoundatLocation 0 (Transformation|GetActorLocation) "0, 0, 0" 0.3 (Math|Random|RandomFloatinRange 0.5 1.5) 0.0 0 0 0)
  (bind _output_get (Variables|Default|SetZombieAnimInstance (Components|SkeletalMesh|GetAnimInstance (Variables|Default|GetZombieHand))))
  (Variables|Default|SetZombieMontage (Animation|Montage|GetCurrentActiveMontage _output_get))
  ;[1 1 1] Hint: Use these nodes to create the material flash when hand is hit
  (bind _returnvalue (Rendering|Material|CreateDynamicMaterialInstance (Variables|Default|GetZombieHand) 0 0 "ZombieHandMat" :!class /Script/Engine.PrimitiveComponent))
  (Variables|Default|SetHandMat _returnvalue))

(fn ConstructionScript)