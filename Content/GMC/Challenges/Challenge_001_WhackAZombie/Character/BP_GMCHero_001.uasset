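; Player hero for the Whack-A-Zombie challenge, with most attack logic driven from C++.
; When the weapon collision overlaps another actor, it plays a sword hit sound there and calls OnHit if that actor is a zombie hand.
; Celebrate spawns a camera at VictoryCamPosition, makes it the player's view target and loops a win animation on the mesh.
; A swing sound node is present but unconnected.
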(event OnComponentBeginOverlap(WeaponCollision)
  (params (OverlappedComponent :type Primitive%20Component%20Object%20Reference) (OtherActor :type Actor%20Object%20Reference) (OtherComp :type Primitive%20Component%20Object%20Reference) (OtherBodyIndex :type Integer) (bFromSweep :type Boolean) (SweepResult :type Hit%20Result%20Structure%20%28by%20ref%29))
  (if (!= OtherActor self)
    (Audio|PlaySoundatLocation "/Game/GMC/GlobalAssets/Audio/SFX/sword_hit.sword_hit" (Transformation|GetActorLocation OtherActor) "0, 0, 0" 1.0 1.0 0.0 0 0 0)
    (bind _asbp_zombie_hand (Utilities|Casting|CastToBP_ZombieHand OtherActor))
    (Default|OnHit _asbp_zombie_hand)))

(event Custom|Celebrate
  (bind _returnvalue (Game|SpawnActorfromClass "/Script/Engine.CameraActor" (Transformation|GetWorldTransform (Variables|Default|GetVictoryCamPosition)) "Undefined" (Game|GetPlayerController 0) 0))
  (Game|Player|SetViewTargetwithBlend (Game|GetPlayerController 0) _returnvalue 0.0 "VTBlend_Linear" 0.0 false)
  (Components|Animation|PlayAnimation (Variables|Character|GetMesh) "/Game/GMC/GlobalAssets/Characters/Animations/Snowball/Anim_Win_Snowball.Anim_Win_Snowball" true))

(event Input|ActionEvents|InputActionAttack
  (params (Key :type Key%20Structure :default "None"))
  ;[1 1 1] Most of the attack logic driven through C++
)

(fn ConstructionScript
  (|CallParentFunction))