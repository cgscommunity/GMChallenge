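; BP_Snowman is an interactable snowman for the SnowToss challenge that opens a dialogue box when the hero interacts with it.
; It forwards pop-up show, hide and interact calls to GMCInteractable.
; Interact hides the HUD and pop-up, then adds a typewriter-paced WBP_002_DialogueBox to the viewport.
; Hiding the pop-up mid-interaction auto-completes the dialogue, restores the HUD and resets the interaction state.
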(event EventBeginPlay)

(event Collision|EventActorBeginOverlap
  (params (OtherActor :type Actor%20Object%20Reference)))

(event Collision|EventActorEndOverlap
  (params (OtherActor :type Actor%20Object%20Reference)))

(fn ConstructionScript)

(fn DisplayInteractPopUp
  (Class|GMCInteractableComponent|CallDisplayPopUp (Variables|Default|GetGMCInteractable))
  (return false))

(fn HideInteractPopUp
  (Class|GMCInteractableComponent|CallHidePopUp (Variables|Default|GetGMCInteractable))
  (if (Variables|Default|GetbInteracting)
    (Default|AutoComplete (Variables|Default|GetDialogueWidget))
    (Class|GMCGameMode|ShowHUD (Variables|/Script/GMChallenge.GMCInteractableComponent|GetGameMode (Variables|Default|GetGMCInteractable)))
    (Variables|Default|SetbInteracting false)
    (Variables|Default|SetGMCHero 0)
    (Variables|Default|SetDialogueWidget 0)
    (Variables|Default|SetCanInteract true)
    (return false)
    (else
      (Variables|Default|SetCanInteract true)
      (return false))))

(fn Interact
  (params (CallingActor :type Actor%20Object%20Reference))
  (if (Variables|Default|GetCanInteract)
    (bind _asbp_gmchero (Utilities|Casting|CastToBP_GMCHero CallingActor))
    (Variables|Default|SetGMCHero _asbp_gmchero)
    (Class|GMCInteractableComponent|CallInteract (Variables|Default|GetGMCInteractable))
    (Class|GMCGameMode|HideHUD (Variables|/Script/GMChallenge.GMCInteractableComponent|GetGameMode (Variables|Default|GetGMCInteractable)))
    (CallFunction|HideInteractPopUp)
    (bind _asbp_gmcplayer_controller (Utilities|Casting|CastToBP_GMCPlayerController (Game|GetPlayerController 0)))
    (bind _returnvalue (UserInterface|CreateWidget "/Game/GMC/Challenges/Challenge_002_SnowToss/UI/WBP_002_DialogueBox.WBP_002_DialogueBox_C" _asbp_gmcplayer_controller))
    (bind _output_get (Variables|Default|SetDialogueWidget _returnvalue))
    (UserInterface|Viewport|AddtoViewport _returnvalue 0)
    (Variables|Default|SetCanInteract false)
    (Variables|Default|SetbInteracting true)
    (return self)))