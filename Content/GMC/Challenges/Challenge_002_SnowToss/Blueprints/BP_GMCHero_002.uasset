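; Player hero for the SnowToss challenge (Challenge 002), extending a parent hero with camera-view switching and dialogue skipping.
; The DialogueAutoComplete input calls CallDialogueAutoComplete to finish dialogue.
; SwitchToFirstPerson pulls the boom past the pivot, centers the camera, hides the actor and sets a fixed control yaw.
; SwitchToThirdPerson extends the boom, applies a sideways camera offset and shows the actor again.
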(event Input|ActionEvents|InputActionDialogueAutoComplete
  (params (Key :type Key%20Structure :default "None"))
  ;[1 1 1] Right Click to Auto Complete Dialogue
  (:Pressed
    (Default|CallDialogueAutoComplete)))

(fn ConstructionScript
  (|CallParentFunction))

(fn SwitchtoFirstPerson
  (Variables|/Script/Engine.SpringArmComponent|SetTargetArmLength (Variables|Default|GetCameraBoom) -2e+01)
  (Transformation|SetRelativeLocation (Variables|Default|GetFollowCamera) "0, 0, 0" false false)
  (Rendering|SetActorHiddenInGame true)
  (Pawn|SetControlRotation (Game|GetPlayerController 0) (Math|Rotator|MakeRotator 0.0 0.0 9e+01)))

(fn SwitchtoThirdPerson
  (Variables|/Script/Engine.SpringArmComponent|SetTargetArmLength (Variables|Default|GetCameraBoom) 4e+02)
  (Transformation|SetRelativeLocation (Variables|Default|GetFollowCamera) "0,50.000000, 0" false false)
  (Rendering|SetActorHiddenInGame false))